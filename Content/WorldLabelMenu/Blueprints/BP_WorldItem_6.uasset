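; BP_WorldItem_6 is a world item that shows an assignable static mesh and labels it with spawned BP_LabelMarker actors.
; The construction script applies the chosen mesh.
; On BeginPlay, socket labeling attaches one marker per mesh socket, using the socket's tag as far name and its name as near details.
; Otherwise, a single marker attaches to the mesh with the item's own name and details text.
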(event `self.ReceiveBeginPlay`
  (bind _staticmeshitem (`self.StaticMeshItem`))
  (if (`self.UseSocketsLabel`)
    (for _array_element (`SceneComponent.GetAllSocketNames` _staticmeshitem)
      (bind _tag (`StaticMeshSocket.Tag` (`StaticMesh.FindSocket` (`StaticMeshComponent.StaticMesh` _staticmeshitem) _array_element)))
      (bind _returnvalue (`|SpawnActorFromClass` "/Game/WorldLabelMenu/Blueprints/BP_LabelMarker.BP_LabelMarker_C" (`KismetMathLibrary.MakeTransform` (0.0 0.0 0.0)) "Undefined" "OverrideRootScale" null (`KismetTextLibrary.Conv_StringToText` (`KismetMathLibrary.SelectString` _tag "" (`KismetStringLibrary.NotEqual_StrStr` _tag))) (`KismetTextLibrary.Conv_NameToText` _array_element) null))
      (`self.K2_AttachToComponent` _returnvalue (`self.StaticMeshItem`) _array_element "KeepRelative" "KeepRelative" "KeepRelative" true))
    (else
      (bind _returnvalue_2 (`|SpawnActorFromClass` "/Game/WorldLabelMenu/Blueprints/BP_LabelMarker.BP_LabelMarker_C" (`KismetMathLibrary.MakeTransform` (0.0 0.0 0.0)) "Undefined" "OverrideRootScale" null (`self.ItemName_Far`) (`self.ItemDetails_Near`) null))
      (`self.K2_AttachToComponent` _returnvalue_2 (`self.StaticMeshItem`) "None" "KeepRelative" "KeepRelative" "KeepRelative" true))))

(fn `UserConstructionScript`
  (`StaticMeshComponent.SetStaticMesh` (`self.StaticMeshItem`) (`self.StaticMeshItemAssign`)))