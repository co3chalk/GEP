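; Ending door actor that picks its gate mesh according to whether all four keys in the game mode are collected.
; On BeginPlay it casts the game mode, stores it, and combines the four key flags with an integer bitwise AND.
; The result selects one of two gate meshes and prints a debug string.
; The check runs only once; overlap and Tick events are empty.
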(event `self.ReceiveBeginPlay`
  (bind _asmy_game_mode_base_bp (cast `/Game/Blueprints/MyGameModeBase_BP` (`GameplayStatics.GetGameMode`)))
  (set `self.mygamemode` _asmy_game_mode_base_bp)
  (`KismetSystemLibrary.PrintString` "Hello")
  (if (`KismetMathLibrary.Conv_IntToBool` (`KismetMathLibrary.And_IntInt` (`KismetMathLibrary.Conv_BoolToInt` (`PrototypeGameMode.HasGotKey_Get` (`self.mygamemode`) 0)) (`KismetMathLibrary.Conv_BoolToInt` (`PrototypeGameMode.HasGotKey_Get` (`self.mygamemode`) 1)) (`KismetMathLibrary.Conv_BoolToInt` (`PrototypeGameMode.HasGotKey_Get` (`self.mygamemode`) 2)) (`KismetMathLibrary.Conv_BoolToInt` (`PrototypeGameMode.HasGotKey_Get` (`self.mygamemode`) 3))))
    (`KismetSystemLibrary.PrintString` "true")
    (`StaticMeshComponent.SetStaticMesh` (`self.StaticMeshComponent`) "/Game/OlbertsLowPolyDungeon/Meshes/DungeonParts/SM_Gate_01.SM_Gate_01")
    (else
      (`KismetSystemLibrary.PrintString` "no")
      (`StaticMeshComponent.SetStaticMesh` (`self.StaticMeshComponent`) "/Game/OlbertsLowPolyDungeon/Meshes/DungeonParts/SM_Gate_02.SM_Gate_02"))))

(fn `UserConstructionScript`)